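; An actor component that applies manual, fake gravity to its owning actor.
; Each tick it adds downward acceleration to a stored velocity and moves the owner by that velocity with a swept world offset.
; When the sweep hits something, it zeroes the vertical velocity and keeps the horizontal part.
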(event EventBeginPlay)

(event EventTick
  (params (DeltaSeconds :type Float%20%28single-precision%29))
  ;[1 1 1] Apply the "fake gravity"
  (bind _output_get (Variables|Default|SetCharacter%20Velocity (+ (Math|Vector|MakeVector 0.0 0.0 (* DeltaSeconds -9.8e+02)) (Variables|Default|GetCharacter%20Velocity))))
  (bind _sweephitresult (Transformation|AddActorWorldOffset (Components|GetOwner) (* _output_get DeltaSeconds) true))
  ;[1 1 1] Null vertical velocity, in case of collision
  (if (.bBlockingHit (Collision|BreakHitResult _sweephitresult))
    (Variables|Default|SetCharacter%20Velocity (* (Variables|Default|GetCharacter%20Velocity) "1.000000,1.000000,0.000000"))))
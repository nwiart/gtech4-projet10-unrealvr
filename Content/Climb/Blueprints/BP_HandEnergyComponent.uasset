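; Hand stamina component for climbing: energy drains while the hand is holding and recovers at the same rate when it is not.
; Tick updates and clamps EnergyLevel between zero and one, then feeds its inverse into the "Stress" parameter of a dynamic M_Hand material on the hand mesh.
; BeginPlay also adds a WB_FlatModeHUD to the viewport, but the left and right energy bar updates are unconnected.
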(event EventBeginPlay
  (bind _returnvalue (Rendering|Material|CreateDynamicMaterialInstance (Variables|Default|GetHand%20Mesh%20Component) 0 "/Game/Climb/Materials/M_Hand.M_Hand" "None" :!class /Script/Engine.PrimitiveComponent))
  (Variables|Default|SetDynamic%20Material _returnvalue)
  (bind _returnvalue_2 (UserInterface|CreateWidget "/Game/Climb/UI/WB_FlatModeHUD.WB_FlatModeHUD_C"))
  (bind _output_get (Variables|Default|SetAltitudeUIRef _returnvalue_2))
  (UserInterface|Viewport|AddtoViewport _output_get 0))

(event EventTick
  (params (DeltaSeconds :type Float%20%28single-precision%29))
  (bind _returnvalue (* DeltaSeconds 0.1))
  (Utilities|FlowControl|Sequence
    (:then_0
      (bind _output_get (Variables|Default|SetEnergy%20Level (+ (Variables|Default|GetEnergy%20Level) (Math|Float|SelectFloat (* _returnvalue -1.0) _returnvalue (Variables|Default|GetIs%20Holding)))))
      (if (<= _output_get 0.0)
        (Variables|Default|SetEnergy%20Level 0.0)
        (elif (>= _output_get 1.0)
          (Variables|Default|SetEnergy%20Level 1.0))))
    (:then_1
      (Rendering|Material|SetScalarParameterValue (Variables|Default|GetDynamic%20Material) "Stress" (- 1.0 (Variables|Default|GetEnergy%20Level)) :!class /Script/Engine.MaterialInstanceDynamic))))
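; First-person flat-mode climbing character that grabs tagged holds with alternating hands, climbs ledges and throws spears.
; A camera sphere trace finds and highlights holds; while hanging, Tick applies a damped spring through LaunchCharacter toward the hold, offset by move input.
; A Free/Hanging/Raising state drives movement, with a timeline lifting the player over ledges.
; Hand energy components and peak altitude score feed the HUD.
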(event OnEnergyUpdate(HandEnergyL)
  (params (Energy :type Float%20%28double-precision%29))
  ;[0.01338 1 0] HUD Energy Update
  (Progress|SetPercent (Variables|/Game/Climb/UI/WB_FlatModeHUD.WB_FlatModeHUD_C|GetEnergyLeftHand (Variables|Default|GetAltitudeUIRef)) Energy))

(event OnEnergyUpdate(HandEnergyR)
  (params (Energy :type Float%20%28double-precision%29))
  ;[0.01338 1 0] HUD Energy Update
  (Progress|SetPercent (Variables|/Game/Climb/UI/WB_FlatModeHUD.WB_FlatModeHUD_C|GetEnergyRightHand (Variables|Default|GetAltitudeUIRef)) Energy))

(event Input|EnhancedActionEvents|EnhancedInputActionIA_Look
  (params (ActionValue :type Vector%202D%20Structure) (ElapsedSeconds :type Float%20%28double-precision%29) (TriggeredSeconds :type Float%20%28double-precision%29) (InputAction :type Input%20Action%20Object%20Reference :default "/Game/Climb/Input/Action/IA_Look.IA_Look"))
  (bind _returnvalue (Game|GetPlayerController 0))
  (bind (_x _y) (Math|Vector2D|BreakVector2D ActionValue))
  ;[1 1 1] Move & Look controls
  (Class|PlayerController|AddYawInput _returnvalue _x)
  (Class|PlayerController|AddPitchInput _returnvalue _y))

(event Input|EnhancedActionEvents|EnhancedInputActionIA_Move
  (params (ActionValue :type Vector%202D%20Structure) (ElapsedSeconds :type Float%20%28double-precision%29) (TriggeredSeconds :type Float%20%28double-precision%29) (InputAction :type Input%20Action%20Object%20Reference :default "/Game/Climb/Input/Action/IA_Move.IA_Move"))
  (bind (_x _y) (Math|Vector2D|BreakVector2D ActionValue))
  (bind _returnvalue (Transformation|GetActorRightVector))
  (bind _returnvalue_2 (* _returnvalue _y))
  ;[1 1 1] Move & Look controls
  (:Triggered
    (switch Utilities|FlowControl|Switch|SwitchonEPlayerState (Variables|Default|GetPlayer%20State)
      (:NewEnumerator0
        (Pawn|Input|AddMovementInput (+ (* (Transformation|GetActorForwardVector) _x) _returnvalue_2) 1.0 false))
      (:NewEnumerator1
        (Variables|Default|SetPull (* (+ (* (Transformation|GetActorUpVector) _x) _returnvalue_2) 8e+01)))))
  (:Canceled
    (Variables|Default|SetPull "0, 0, 0" :!label _label))
  (:Completed
    (goto _label)))

(event Input|EnhancedActionEvents|EnhancedInputActionIA_ClimbLedge
  (params (ActionValue :type Boolean) (ElapsedSeconds :type Float%20%28double-precision%29) (TriggeredSeconds :type Float%20%28double-precision%29) (InputAction :type Input%20Action%20Object%20Reference :default "/Game/Climb/Input/Action/IA_ClimbLedge.IA_ClimbLedge"))
  ;[1 1 1] Climb up & Drop down
  (if (> (.X (Math|Vector2D|BreakVector2D (Input|EnhancedActionValues|GetIA_Move))) 0.5)
    (bind _asbp_climbing_ledge (Utilities|Casting|CastToBP_ClimbingLedge (Components|GetOwner (Variables|Default|GetHold%20Component))))
    (Variables|Default|SetPlayer%20State "NewEnumerator2")
    (Variables|/Game/Climb/Blueprints/BP_HandEnergyComponent.BP_HandEnergyComponent_C|SetIs%20Holding (Variables|Default|GetHandEnergyL) false)
    (Variables|/Game/Climb/Blueprints/BP_HandEnergyComponent.BP_HandEnergyComponent_C|SetIs%20Holding (Variables|Default|GetHandEnergyR) false)
    ;;[1 1 1] Transition player up the ledge
    (Variables|Default|SetPrevious%20Location (Transformation|GetActorLocation))
    (bind (_direction _height _forward) (Timeline|Go%20up PlayFromStart)
      (:Update
        (Transformation|SetActorLocation (Math|Vector|MakeVector (Math|Float|Lerp (.x (Variables|Default|GetPrevious%20Location)) (.x (Transformation|GetWorldLocation (Variables|/Game/Climb/Blueprints/BP_ClimbingLedge.BP_ClimbingLedge_C|GetArrow _asbp_climbing_ledge))) _forward) (Math|Float|Lerp (.y (Variables|Default|GetPrevious%20Location)) (.y (Transformation|GetWorldLocation (Variables|/Game/Climb/Blueprints/BP_ClimbingLedge.BP_ClimbingLedge_C|GetArrow _asbp_climbing_ledge))) _forward) (Math|Float|Lerp (.z (Variables|Default|GetPrevious%20Location)) (+ (.z (Transformation|GetWorldLocation (Variables|/Game/Climb/Blueprints/BP_ClimbingLedge.BP_ClimbingLedge_C|GetArrow _asbp_climbing_ledge))) (Variables|/Script/Engine.CapsuleComponent|GetCapsuleHalfHeight (Variables|Collision|GetCapsuleComponent))) _height)) false true))
      (:Finished
        (CallFunction|ResetHandPositions)
        (Variables|Default|SetHold%20Component 0)
        (Variables|Default|SetPlayer%20State "NewEnumerator0")))))

(event Input|EnhancedActionEvents|EnhancedInputActionIA_Drop
  (params (ActionValue :type Boolean) (ElapsedSeconds :type Float%20%28double-precision%29) (TriggeredSeconds :type Float%20%28double-precision%29) (InputAction :type Input%20Action%20Object%20Reference :default "/Game/Climb/Input/Action/IA_Drop.IA_Drop"))
  ;[1 1 1] Climb up & Drop down
  (if (< (.X (Math|Vector2D|BreakVector2D (Input|EnhancedActionValues|GetIA_Move))) -0.5)
    (Variables|Default|SetHold%20Component 0)
    (Variables|Default|SetPlayer%20State "NewEnumerator0")
    (CallFunction|ResetHandPositions)
    (Variables|/Game/Climb/Blueprints/BP_HandEnergyComponent.BP_HandEnergyComponent_C|SetIs%20Holding (Variables|Default|GetHandEnergyL) false)
    (Variables|/Game/Climb/Blueprints/BP_HandEnergyComponent.BP_HandEnergyComponent_C|SetIs%20Holding (Variables|Default|GetHandEnergyR) false)))

(event EventBeginPlay
  (Input|AddMappingContext (PlayerController|LocalPlayerSubsystems|GetEnhancedInputLocalPlayerSubsystem (Game|GetPlayerController 0)) "/Game/Climb/Input/IMC_FlatMode.IMC_FlatMode" 0 "(bIgnoreAllPressedKeysUntilRelease=True,bForceImmediately=False,bNotifyUserSettings=False)")
  (Variables|Default|SetHand%20Rest%20Location%20L (Variables|/Script/Engine.SceneComponent|GetRelativeLocation (Variables|Default|GetHandLeft)))
  (Variables|Default|SetHand%20Rest%20Location%20R (Variables|/Script/Engine.SceneComponent|GetRelativeLocation (Variables|Default|GetHandRight)))
  (Variables|Default|SetSetInitialZ (.z (Transformation|GetActorLocation)))
  (bind _returnvalue (UserInterface|CreateWidget "/Game/Climb/UI/WB_FlatModeHUD.WB_FlatModeHUD_C"))
  (bind _output_get (Variables|Default|SetAltitudeUIRef _returnvalue))
  (UserInterface|Viewport|AddtoViewport _output_get 0)
  (Variables|/Script/UMG.TextBlock|SetText (Variables|/Game/Climb/UI/WB_FlatModeHUD.WB_FlatModeHUD_C|GetScoreText _output_get) "0"))

(event EventPossessed
  (params (NewController :type Controller%20Object%20Reference))
  (bind _returnvalue (UserInterface|CreateWidget "/Game/Climb/UI/WB_FlatModeHUD.WB_FlatModeHUD_C"))
  (UserInterface|Viewport|AddtoViewport _returnvalue 0))

(event EventTick
  (params (DeltaSeconds :type Float%20%28single-precision%29))
  (bind _hold_component (Variables|Default|GetHold%20Component))
  (Utilities|FlowControl|Sequence
    (:then_0
      (Utilities|IsValid _hold_component
        (:Is%20Valid
          (if (Utilities|Enum|Equal(Enum) (Variables|Default|GetPlayer%20State) "NewEnumerator1")
            (Character|LaunchCharacter (+ (* (- (Transformation|GetWorldLocation _hold_component) (Transformation|GetWorldLocation (select (Variables|Default|GetRight%20Hand) (Variables|Default|GetGrabPosR) (Variables|Default|GetGrabPosL)))) 4.0) (* (Variables|/Script/Engine.MovementComponent|GetVelocity (Variables|Character|GetCharacterMovement)) -0.4) (Variables|Default|GetPull)) false false)
            (Transformation|SetWorldLocation (select (Variables|Default|GetRight%20Hand) (Variables|Default|GetHandRight) (Variables|Default|GetHandLeft)) (Transformation|GetWorldLocation (Variables|Default|GetHold%20Component)) false true)
            (bind _output_get (Variables|Default|SetAltitudeScore (* (Math|Float|Round (Math|Float|Max(Float) (- (.z (Transformation|GetActorLocation)) (Variables|Default|GetSetInitialZ)) 0.0)) (Variables|Default|GetAltitudeMultiplier))))
            (Math|Float|CompareFloat _output_get (Variables|Default|GetMaxAltitudeScore)
              (:>
                (bind _output_get_2 (Variables|Default|SetMaxAltitudeScore (Variables|Default|GetAltitudeScore)))
                (Variables|/Script/UMG.TextBlock|SetText (Variables|/Game/Climb/UI/WB_FlatModeHUD.WB_FlatModeHUD_C|GetScoreText (Variables|Default|GetAltitudeUIRef)) (Utilities|Text|ToText(Float) _output_get_2 "HalfToEven"))))))))
    (:then_1
      ;[1 1 1] Make hovered hold pulse
      (bind _hold_component_2 (CallFunction|GetPointedHold))
      (if (!= _hold_component_2 (Variables|Default|GetHovered%20Hold%20Component))
        (Utilities|FlowControl|Sequence
          (:then_0
            (bind _asmesh_component (Utilities|Casting|CastToMeshComponent (Variables|Default|GetHovered%20Hold%20Component)))
            (Rendering|Material|SetOverlayMaterial _asmesh_component 0 :!class /Script/Engine.MeshComponent))
          (:then_1
            (bind _output_get_3 (Variables|Default|SetHovered%20Hold%20Component _hold_component_2))
            (bind _asmesh_component_2 (Utilities|Casting|CastToMeshComponent _output_get_3))
            (Rendering|Material|SetOverlayMaterial _asmesh_component_2 "/Game/Climb/Materials/M_HoldOverlay.M_HoldOverlay" :!class /Script/Engine.MeshComponent)))))))

(event Input|MouseEvents|RightMouseButton
  (params (Key :type Key%20Structure :default "None"))
  (:Released
    (Utilities|IsValid (Variables|Default|GetThrowable%20Object)
      (:Is%20Valid
        (bind _asbp_spear (Utilities|Casting|CastToBP_Spear (Variables|Default|GetThrowable%20Object)))
        (Default|Throw _asbp_spear (* (Math|Vector|GetForwardVector (Variables|Default|GetCamera)) 1e+03))
        (Variables|Default|SetThrowable%20Object 0)))))

(event Input|MouseEvents|LeftMouseButton
  (params (Key :type Key%20Structure :default "None"))
  ;[1 1 1] Climbing hold grab
  (:Pressed
    (Variables|Default|SetRight%20Hand (not (Variables|Default|GetRight%20Hand)))
    (Variables|/Game/Climb/Blueprints/BP_HandEnergyComponent.BP_HandEnergyComponent_C|SetIs%20Holding (Variables|Default|GetHandEnergyL) false)
    (Variables|/Game/Climb/Blueprints/BP_HandEnergyComponent.BP_HandEnergyComponent_C|SetIs%20Holding (Variables|Default|GetHandEnergyR) false)
    (bind _hold_component (CallFunction|GetPointedHold))
    (Utilities|IsValid _hold_component
      (:Is%20Valid
        (Variables|/Game/Climb/Blueprints/BP_HandEnergyComponent.BP_HandEnergyComponent_C|SetIs%20Holding (select (Variables|Default|GetRight%20Hand) (Variables|Default|GetHandEnergyR) (Variables|Default|GetHandEnergyL)) true)
        (if (!= (Variables|Default|GetHold%20Component) _hold_component)
          (Variables|Default|SetHold%20Component _hold_component)
          (Variables|Default|SetPlayer%20State "NewEnumerator1")
          (CallFunction|ResetHandPositions)
          (bind _asbp_hold_falling (Utilities|Casting|CastToBP_HoldFalling (Components|GetOwner (Variables|Default|GetHold%20Component))))
          (Default|NotifyGrabbed _asbp_hold_falling self))))))

(event Input|KeyboardEvents|E
  (params (Key :type Key%20Structure :default "None"))
  (bind _camera (Variables|Default|GetCamera))
  (bind _returnvalue (Transformation|GetWorldLocation _camera))
  (:Pressed
    (bind (_outhit _returnvalue_2) (Collision|SphereTraceForObjects _returnvalue (+ _returnvalue (* (Math|Vector|GetForwardVector _camera) (Variables|Default|GetMax%20Grab%20Range))) 5e+01 (Utilities|Array|MakeArray "ObjectTypeQuery6") false 0 "None" true "(R=0.000000,G=1.000000,B=1.000000,A=1.000000)" "(R=0.000000,G=1.000000,B=0.000000,A=1.000000)" 1.0))
    (if _returnvalue_2
      (if (Actor|ActorHasTag (.HitActor (Collision|BreakHitResult _outhit)) (Variables|Default|GetGrab%20Obj%20Tag))
        (bind _output_get (Variables|Default|SetThrowable%20Object (.HitActor (Collision|BreakHitResult _outhit))))
        (Transformation|AttachComponentToComponent _output_get (Variables|Default|GetHandRight) "None" "SnapToTarget" "KeepRelative" "KeepRelative" true)
        (bind _asbp_spear (Utilities|Casting|CastToBP_Spear _output_get))
        (Collision|SetCollisionEnabled (Variables|/Game/Climb/Blueprints/BP_Spear.BP_Spear_C|GetCylinder _asbp_spear) "NoCollision")))))

(fn ConstructionScript
  (Variables|/Game/Climb/Blueprints/BP_HandEnergyComponent.BP_HandEnergyComponent_C|SetHand%20Mesh%20Component (Variables|Default|GetHandEnergyL) (Variables|Default|GetHandLeft))
  (Variables|/Game/Climb/Blueprints/BP_HandEnergyComponent.BP_HandEnergyComponent_C|SetHand%20Mesh%20Component (Variables|Default|GetHandEnergyR) (Variables|Default|GetHandRight)))

(fn GetPointedHold
  (bind _camera (Variables|Default|GetCamera))
  (bind _returnvalue (Transformation|GetWorldLocation _camera))
  (bind (_outhit _returnvalue_2) (Collision|SphereTraceForObjects _returnvalue (+ _returnvalue (* (Math|Vector|GetForwardVector _camera) (Variables|Default|GetMax%20Grab%20Range))) 5.0 (Utilities|Array|MakeArray "ObjectTypeQuery4") false 0 "None" true "(R=0.000000,G=1.000000,B=1.000000,A=1.000000)" "(R=0.000000,G=1.000000,B=0.000000,A=1.000000)" 1.0))
  (if _returnvalue_2
    (if (Actor|ActorHasTag (.HitActor (Collision|BreakHitResult _outhit)) (Variables|Default|GetClimb%20Hold%20Tag))
      (return (.HitComponent (Collision|BreakHitResult _outhit)))
      (else
        _)))
  (return 0))

(fn ResetHandPositions
  (Transformation|SetRelativeLocation (Variables|Default|GetHandRight) (Variables|Default|GetHand%20Rest%20Location%20R) false true)
  (Transformation|SetRelativeLocation (Variables|Default|GetHandLeft) (Variables|Default|GetHand%20Rest%20Location%20L) false true))

(fn ReleaseHolds
  (Variables|Default|SetHold%20Component 0)
  (Variables|Default|SetPlayer%20State "NewEnumerator0")
  (CallFunction|ResetHandPositions)
  (Variables|/Game/Climb/Blueprints/BP_HandEnergyComponent.BP_HandEnergyComponent_C|SetIs%20Holding (Variables|Default|GetHandEnergyL) false)
  (Variables|/Game/Climb/Blueprints/BP_HandEnergyComponent.BP_HandEnergyComponent_C|SetIs%20Holding (Variables|Default|GetHandEnergyR) false))
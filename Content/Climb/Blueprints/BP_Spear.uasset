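; BP_Spear is a throwable spear that becomes a climbing hold where it lands.
; Throw detaches it, clears its tags and launches the physics-simulated cylinder, while Tick points its Z axis along the velocity.
; On hit, it stops physics and ticking, aligns to the surface normal and gains the ClimbHold tag.
; A timeline then scales a sine yaw wobble, offsetting location so the spear jiggles about its impact point.
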(event OnComponentHit(Cylinder)
  (params (HitComponent :type Primitive%20Component%20Object%20Reference) (OtherActor :type Actor%20Object%20Reference) (OtherComp :type Primitive%20Component%20Object%20Reference) (NormalImpulse :type Vector :default "0, 0, 0") (Hit :type Hit%20Result%20Structure%20%28by%20ref%29))
  (bind (_bblockinghit _binitialoverlap _time _distance _location _impactpoint _normal _impactnormal) (Collision|BreakHitResult Hit))
  (Physics|SetSimulatePhysics (Variables|Default|GetCylinder) false)
  (bind _output_get (Variables|Default|SetLocation (+ _impactpoint (* _impactnormal 5e+01))))
  (bind _output_get_2 (Variables|Default|SetRotation (Math|Rotator|MakeRotfromZ (Math|Vector|NegateVector _impactnormal))))
  (Variables|Default|SetDir%20Vector (Math|Vector|GetUpVector _output_get_2))
  (Transformation|SetActorLocationAndRotation _output_get _output_get_2 false true)
  (Actor|Tick|SetActorTickEnabled false)
  (Variables|Default|SetTags (Utilities|Array|MakeArray "ClimbHold"))
  ;[1 1 1] Animate spear to jiggle once it lands
  (bind _oscillation_amplitude (Timeline|Prrrrrrr PlayFromStart)
    (:Update
      (Transformation|SetActorLocationAndRotation (+ (* (- (Variables|Default|GetDir%20Vector) (Math|Vector|GetUpVector (Math|Rotator|MakeRotator (.roll (Variables|Default|GetRotation)) (.pitch (Variables|Default|GetRotation)) (+ (.yaw (Variables|Default|GetRotation)) (* _oscillation_amplitude (Math|Trig|Sin(Radians) (* (Actor|GetGameTimeSinceCreation) 1e+02)) 1e+01))))) 5e+01) (Variables|Default|GetLocation)) (Math|Rotator|MakeRotator (.roll (Variables|Default|GetRotation)) (.pitch (Variables|Default|GetRotation)) (+ (.yaw (Variables|Default|GetRotation)) (* _oscillation_amplitude (Math|Trig|Sin(Radians) (* (Actor|GetGameTimeSinceCreation) 1e+02)) 1e+01))) false true))))

(event EventBeginPlay)

(event Collision|EventActorBeginOverlap
  (params (OtherActor :type Actor%20Object%20Reference)))

(event EventTick
  (params (DeltaSeconds :type Float%20%28single-precision%29))
  (bind _cylinder (Variables|Default|GetCylinder))
  (if (Physics|IsSimulatingPhysics _cylinder "None")
    (bind _returnvalue (Physics|GetPhysicsLinearVelocity _cylinder "None"))
    (Transformation|SetActorRotation (Math|Rotator|MakeRotfromZ _returnvalue))))

(fn ConstructionScript)

(fn Throw
  (params (Velocity :type Vector))
  (bind _cylinder (Variables|Default|GetCylinder))
  (Transformation|DetachFromComponent (Variables|Transformation|GetRootComponent) "KeepWorld" "KeepWorld" "KeepWorld" true)
  (Collision|SetCollisionEnabled _cylinder "QueryAndPhysics")
  (Physics|SetSimulatePhysics _cylinder true)
  (Physics|SetPhysicsLinearVelocity _cylinder Velocity false "None")
  (Utilities|Array|Clear (Variables|Actor|GetTags)))
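; BP_HoldFalling is a climbing hold that falls a set delay after a player grabs it.
; The grab notification stores the player and starts a one-shot timer that calls Fall.
; Fall enables physics on the Cylinder, clears the actor's tags and sets a short lifespan.
; If the player's HoldComponent is still that Cylinder, it also makes them release their holds.
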(event Custom|Notify%20Grabbed
  (params (Player :type BP%20Flat%20Mode%20Character%20Object%20Reference))
  (Variables|Default|SetPlayer%20Ref Player)
  (Utilities|Time|SetTimerbyEvent (delegate Custom|Fall) (Variables|Default|GetTime%20Before%20Falling)))

(event Custom|Fall
  (bind _player_ref (Variables|Default|GetPlayer%20Ref))
  (Physics|SetSimulatePhysics (Variables|Default|GetCylinder) true)
  (Utilities|Array|Clear (Variables|Actor|GetTags))
  (Actor|SetLifeSpan 5.0)
  (if (== (Variables|/Game/Climb/Blueprints/BP_FlatModeCharacter.BP_FlatModeCharacter_C|GetHold%20Component _player_ref) (Variables|Default|GetCylinder))
    (Default|ReleaseHolds _player_ref)))

(event EventBeginPlay)

(event EventTick
  (params (DeltaSeconds :type Float%20%28single-precision%29)))

(fn ConstructionScript)